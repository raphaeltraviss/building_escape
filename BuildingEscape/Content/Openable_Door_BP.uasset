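; Openable door actor that swings open and closed when its OpenDoor events fire.
; BeginPlay caches the initial rotation and location, then a timeline plays on open and reverses on close, adding its yaw angle to the initial rotation.
; A timeline event track plays a door lock sound at the door's starting location.
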(event `self.ReceiveBeginPlay`
  (set `self.InitialRotation` (`self.K2_GetActorRotation`))
  (set `self.InitialLocation` (`self.K2_GetActorLocation`)))

(event `self.OpenDoor.OnOpen`
  (bind (_direction _open_angle) (`Timeline|Timeline_0` :!label _label)
    (:`Update`
      (`self.K2_SetActorRotation` (`KismetMathLibrary.ComposeRotators` (`KismetMathLibrary.MakeRotator` 0.0 0.0 _open_angle) (`self.InitialRotation`))))
    (:`Sound Timing`
      (`GameplayStatics.PlaySoundAtLocation` "/Game/Audio/door-lock.door-lock" (`self.InitialLocation`) (`self.InitialRotation`)))))

(event `self.OpenDoor.OnClose`
  (goto _label :!via `Reverse`))

(fn `UserConstructionScript`)